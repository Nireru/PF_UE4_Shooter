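; Bot spawn zone actor that spawns BP_Bot actors at random points inside its Zone box until a spawn limit is reached.
; From BeginPlay, a gated loop waits a random delay, lights the Cube's material, spawns a bot, then restores the unlit material after a short pause.
; Each pass increments a counter and re-enters the gate, which closes once the counter equals MaxSpawnValue.
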(event EventBeginPlay
  (Utilities|FlowControl|Gate false :!label _label
    (:Exit
      ;[1 1 1] Spawn Delay
      (Utilities|FlowControl|Delay (Math|Random|RandomFloatinRange (Variables|Default|GetMinSpawnTime) (Variables|Default|GetMaxSpawnTime)))
      (Utilities|Glow
        (:Out
          (Utilities|Spawn
            (:Out
              ;[1 1 1] Close gate if reached spawn limit, otherwise +1 "spawned"
              (Utilities|Unglow
                (:Out
                  (if (== (Variables|Default|GetMaxSpawnValue) (Variables|Default|GetSpawned))
                    (goto _label Close)
                    (else
                      (Math|Integer|IncrementInt (Variables|Default|GetSpawned)
                        (:%20%20
                          (goto _label))))))))))))))

(fn ConstructionScript)