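; BP_Bot_SpawnZone is a zone actor that spawns BPC_Bot actors at random points inside its Zone box.
; From BeginPlay, a self-feeding Gate loop waits a random delay between the min and max spawn times, then spawns with collision adjustment.
; The limit check follows each spawn, incrementing Spawned and looping until it equals MaxSpawnValue, which closes the gate.
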(event EventBeginPlay
  (bind _zone (Variables|Default|GetZone))
  (Development|PrintString "BP_Bot_SpawnZone BeginPlay")
  (Utilities|FlowControl|Gate false :!label _label
    (:Exit
      ;[1 1 1] Spawn Delay
      (Utilities|FlowControl|Delay (Math|Random|RandomFloatinRange (Variables|Default|GetMinSpawnTime) (Variables|Default|GetMaxSpawnTime)))
      ;[1 1 1] Spawn in random place inside box
      (Game|SpawnActorfromClass "/Game/Bot/BPC_Bot.BPC_Bot_C" (Math|Conversions|ToTransform(Vector) (Math|Random|RandomPointinBoundingBox (Transformation|GetWorldLocation _zone) (Components|Box|GetScaledBoxExtent _zone))) "AdjustIfPossibleButDontSpawnIfColliding" 0 0)
      ;[1 1 1] Close gate if reached spawn limit, otherwise +1 "spawned"
      (if (== (Variables|Default|GetMaxSpawnValue) (Variables|Default|GetSpawned))
        (goto _label Close)
        (else
          (Math|Integer|IncrementInt (Variables|Default|GetSpawned)
            (:%20%20
              (goto _label))))))))

(fn ConstructionScript)