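; Space skybox actor that applies a configurable material to its static mesh and sets the look of the space backdrop.
; It writes power, scene brightness and star brightness values into the MP_Space_Skybox material parameter collection.
; The same setup runs in both the construction script and BeginPlay, so it applies at construction and again when play starts.
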(event EventBeginPlay
  (Rendering|Material|SetMaterial (Variables|Default|GetStaticMesh) 0 (Variables|Default|GetMaterial))
  (Rendering|Material|SetScalarParameterValue "/Game/LevelData/Skybox/MP_Space_Skybox.MP_Space_Skybox" "Power" (Variables|Default|GetPower) :!class /Script/Engine.KismetMaterialLibrary)
  (Rendering|Material|SetScalarParameterValue "/Game/LevelData/Skybox/MP_Space_Skybox.MP_Space_Skybox" "Scene brightness" (Variables|Default|GetScene%20brightness) :!class /Script/Engine.KismetMaterialLibrary)
  (Rendering|Material|SetScalarParameterValue "/Game/LevelData/Skybox/MP_Space_Skybox.MP_Space_Skybox" "Star brightness" (Variables|Default|GetStar%20Brighntess) :!class /Script/Engine.KismetMaterialLibrary))

(fn ConstructionScript
  (Rendering|Material|SetMaterial (Variables|Default|GetStaticMesh) 0 (Variables|Default|GetMaterial))
  (Rendering|Material|SetScalarParameterValue "/Game/LevelData/Skybox/MP_Space_Skybox.MP_Space_Skybox" "Power" (Variables|Default|GetPower) :!class /Script/Engine.KismetMaterialLibrary)
  (Rendering|Material|SetScalarParameterValue "/Game/LevelData/Skybox/MP_Space_Skybox.MP_Space_Skybox" "Scene brightness" (Variables|Default|GetScene%20brightness) :!class /Script/Engine.KismetMaterialLibrary)
  (Rendering|Material|SetScalarParameterValue "/Game/LevelData/Skybox/MP_Space_Skybox.MP_Space_Skybox" "Star brightness" (Variables|Default|GetStar%20Brighntess) :!class /Script/Engine.KismetMaterialLibrary))