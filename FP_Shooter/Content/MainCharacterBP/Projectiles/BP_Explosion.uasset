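; BP_Explosion is a short-lived explosion actor in the main character's projectiles that damages bots and pushes physics objects.
; After a brief delay for collision to register, it applies radial damage with falloff once per overlapping BP_Bot, credited to player controller 0, so several bots stack hits.
; It then fires a radial force impulse, destroys its collision component and expires after a few seconds.
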(event EventBeginPlay
  (Utilities|FlowControl|Delay 0.1) ; Delay for collision to be able to spawn
  (for _array_element (Collision|GetOverlappingActors (Variables|Default|GetCollision) "/Game/Bot/BP_Bot.BP_Bot_C" :!class /Script/Engine.PrimitiveComponent)
    (Class|GameplayStatics|ApplyRadialDamagewithFalloff 8e+01 1e+01 (Transformation|GetWorldLocation (Variables|Default|GetOrigin)) 1e+02 8e+02 12.0 0 0 self (Game|GetPlayerController 0) "ECC_Visibility"))
  (Class|RadialForceComponent|FireImpulse (Variables|Default|GetRadialForce))
  (Components|DestroyComponent (Variables|Default|GetCollision))
  (Actor|SetLifeSpan 3.0))

(fn ConstructionScript)