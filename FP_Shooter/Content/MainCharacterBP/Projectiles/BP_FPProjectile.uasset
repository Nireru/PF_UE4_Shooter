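; First-person projectile actor that deals gun damage to actors it overlaps.
; On overlap it reads the player's BPC_FirstPerson to apply primary or secondary gun damage, chosen by whether the secondary is held at impact, then destroys itself.
; A blocking hit destroys it without damage, and a ten-second lifespan limits how long it exists.
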(event OnComponentBeginOverlap(CollisionComponent)
  (params (OverlappedComponent :type Primitive%20Component%20Object%20Reference) (OtherActor :type Actor%20Object%20Reference) (OtherComp :type Primitive%20Component%20Object%20Reference) (OtherBodyIndex :type Integer) (bFromSweep :type Boolean) (SweepResult :type Hit%20Result%20Structure%20%28by%20ref%29))
  (bind _self self)
  (bind _asbpc_first_person (Utilities|Casting|CastToBPC_FirstPerson (Game|GetPlayerCharacter 0)))
  (if (Variables|/Game/MainCharacterBP/BPC_FirstPerson.BPC_FirstPerson_C|GetHoldingSecondary? _asbpc_first_person)
    (Game|Damage|ApplyDamage OtherActor (Variables|/Game/MainCharacterBP/BPC_FirstPerson.BPC_FirstPerson_C|GetSecondaryGun_Damage _asbpc_first_person) 0 _self) ; Secondary gun
    (else
      (Game|Damage|ApplyDamage OtherActor (Variables|/Game/MainCharacterBP/BPC_FirstPerson.BPC_FirstPerson_C|GetPrimaryGun_Damage _asbpc_first_person) 0 _self) ; Primary gun
    ))
  (Actor|DestroyActor))

(event OnComponentHit(CollisionComponent)
  (params (HitComponent :type Primitive%20Component%20Object%20Reference) (OtherActor :type Actor%20Object%20Reference) (OtherComp :type Primitive%20Component%20Object%20Reference) (NormalImpulse :type Vector :default "0, 0, 0") (Hit :type Hit%20Result%20Structure%20%28by%20ref%29))
  (Actor|DestroyActor))

(event EventBeginPlay
  (Actor|SetLifeSpan 1e+01))

(fn ConstructionScript)