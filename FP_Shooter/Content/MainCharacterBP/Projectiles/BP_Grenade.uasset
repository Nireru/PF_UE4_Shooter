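; BP_Grenade is a grenade actor in the main character's projectiles that explodes on a timer or on overlap.
; BeginPlay starts a one-shot timer using the Timer variable, which calls Detonate.
; An overlap on SM_Grenade triggers the same logic early, guarded by a DoOnce.
; Both paths spawn BP_Explosion at the grenade's transform and set a near-zero lifespan to remove the grenade.
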(event OnComponentBeginOverlap(SM_Grenade)
  (params (OverlappedComponent :type Primitive%20Component%20Object%20Reference) (OtherActor :type Actor%20Object%20Reference) (OtherComp :type Primitive%20Component%20Object%20Reference) (OtherBodyIndex :type Integer) (bFromSweep :type Boolean) (SweepResult :type Hit%20Result%20Structure%20%28by%20ref%29))
  ;[1 1 1] Overlap by projectile
  (Utilities|FlowControl|DoOnce false
    (:Completed
      (Actor|SetLifeSpan 0.01)
      (Game|SpawnActorfromClass "/Game/MainCharacterBP/Projectiles/BP_Explosion.BP_Explosion_C" (Transformation|GetActorTransform) "AlwaysSpawn" 0 0))))

(event Custom|Detonate
  ;[1 1 1] Explosion & Explosion timer
  (Actor|SetLifeSpan 0.01)
  (Game|SpawnActorfromClass "/Game/MainCharacterBP/Projectiles/BP_Explosion.BP_Explosion_C" (Transformation|GetActorTransform) "AlwaysSpawn" 0 0))

(event EventBeginPlay
  ;[1 1 1] Explosion & Explosion timer
  (Utilities|Time|SetTimerbyEvent (delegate Custom|Detonate) (Variables|Default|GetTimer)))

(fn ConstructionScript)